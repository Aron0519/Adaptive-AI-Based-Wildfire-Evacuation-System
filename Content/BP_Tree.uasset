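; BP_Tree is a tree actor that can catch fire, burn and then disappear.
; CatchFire, guarded by IsBurning so it only runs once, shows the smoke and fire effects and swaps the static mesh to the burned material.
; After a fixed delay the actor destroys itself; nothing in this Blueprint calls CatchFire, and its BeginPlay, overlap and Tick events are empty.
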(event Custom|CatchFire
  (if (not (Variables|Default|GetIsBurning))
    (Variables|Default|SetIsBurning true)
    (Rendering|SetVisibility (Variables|Default|GetSmokeEffect) true false)
    (Rendering|Material|SetMaterial (Variables|Default|GetStaticMesh) 0 (Variables|Default|GetBurnedMaterial))
    (Rendering|SetVisibility (Variables|Default|GetFireEffect) true false)
    (Utilities|FlowControl|Delay 15.0)
    (Actor|DestroyActor)))

(event EventBeginPlay)

(event Collision|EventActorBeginOverlap
  (params (OtherActor :type Actor%20Object%20Reference)))

(event EventTick
  (params (DeltaSeconds :type Float%20%28single-precision%29)))

(fn ConstructionScript)