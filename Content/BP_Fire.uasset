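; BP_Fire is a fire actor that slowly spreads itself and ignites trees.
; After a long delay from BeginPlay it spawns another BP_Fire at a random nearby horizontal offset, so each fire continues the chain with one successor.
; Its Box overlap casts the other actor to BP_Tree and calls CatchFire on it.
; Nothing in its graphs extinguishes or destroys the fire.
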(event OnComponentBeginOverlap(Box)
  (params (OverlappedComponent :type Primitive%20Component%20Object%20Reference) (OtherActor :type Actor%20Object%20Reference) (OtherComp :type Primitive%20Component%20Object%20Reference) (OtherBodyIndex :type Integer) (bFromSweep :type Boolean) (SweepResult :type Hit%20Result%20Structure%20%28by%20ref%29))
  (bind _asbp_tree (Utilities|Casting|CastToBP_Tree OtherActor))
  (Default|CatchFire _asbp_tree))

(event EventBeginPlay
  (Utilities|FlowControl|Delay 1e+03)
  (Game|SpawnActorfromClass "BP_Fire_C" (Math|Transform|MakeTransform (+ (Math|Vector|MakeVector (Math|Random|RandomFloatinRange -1.5e+02 1.5e+02) (Math|Random|RandomFloatinRange -1.5e+02 1.5e+02) 0.0) (Transformation|GetActorLocation self)) "0, 0, 0" "2.000000,2.000000,1.000000") "Undefined" "MultiplyWithRoot" 0 0))

(event Collision|EventActorBeginOverlap
  (params (OtherActor :type Actor%20Object%20Reference)))

(event EventTick
  (params (DeltaSeconds :type Float%20%28single-precision%29)))

(fn ConstructionScript)